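; BP_LSTrigger is an overlap trigger that starts the game's ending cinematic.
; On overlap it flags the player's cinematic state, destroys an overlapping raft, or freezes an overlapping player and blends to WaveHitCineCamera, then disables its box collision.
; If the hook-aim UI is valid, it removes it and plays EndingSequence.
; When the sequence finishes, it shows the restart widget with mouse cursor and UI-only input.
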(event Custom|SequenceFinish
  (bind _returnvalue (Game|GetPlayerController 0))
  (bind _returnvalue_2 (UserInterface|CreateWidget "/Game/Sequence/WBP_Restart.WBP_Restart_C" _returnvalue))
  (UserInterface|Viewport|AddtoViewport _returnvalue_2 0)
  (Variables|/Script/Engine.PlayerController|SetbShowMouseCursor _returnvalue true)
  (Input|SetInputModeUIOnly _returnvalue _returnvalue_2 "DoNotLock" false))

(event Collision|EventActorBeginOverlap
  (params (OtherActor :type Actor%20Object%20Reference))
  (bind _endingsequence (Variables|Default|GetEndingSequence))
  (bind _sequenceplayer (Variables|/Script/LevelSequence.LevelSequenceActor|GetSequencePlayer _endingsequence))
  (Utilities|FlowControl|Sequence
    (:then_0
      (bind _asbp_my_fpc (Utilities|Casting|CastToBP_MyFPC (Game|GetPlayerCharacter 0)))
      (Variables|/Game/FirstPerson/Blueprints/BP_MyFPC.BP_MyFPC_C|SetbCinematicStart _asbp_my_fpc true))
    (:then_1
      (bind _asbp_raft (Utilities|Casting|CastToBP_Raft OtherActor))
      (Actor|DestroyActor _asbp_raft))
    (:then_2
      (bind _asbp_my_fpc_2 (Utilities|Casting|CastToBP_MyFPC OtherActor))
      (Utilities|FlowControl|DoOnce false
        (:Completed
          (Input|DisableInput _asbp_my_fpc_2 (Pawn|GetLocalViewingPlayerController _asbp_my_fpc_2))
          (Pawn|Components|CharacterMovement|DisableMovement (Variables|/Script/Engine.Character|GetCharacterMovement _asbp_my_fpc_2))
          (Game|Player|SetViewTargetwithBlend (Pawn|GetLocalViewingPlayerController _asbp_my_fpc_2) (Variables|Default|GetWaveHitCineCamera) 0.5 "VTBlend_Linear" 0.0 false))))
    (:then_3
      (EventDispatchers|BindEventtoOnFinished _sequenceplayer (delegate Custom|SequenceFinish))
      (bind _asbp_my_fpc_3 (Utilities|Casting|CastToBP_MyFPC (Game|GetPlayerCharacter 0)))
      (Utilities|IsValid (Variables|/Script/SemiRaft.MyCharacter|GetHookAimUI _asbp_my_fpc_3)
        (:Is%20Valid
          (Class|MyCharacter|RemoveHookAimUI _asbp_my_fpc_3)
          (bind _foundwidgets (Widget|GetAllWidgetsOfClass "/Game/ToolSystem/UI/WBP_HookAimUI.WBP_HookAimUI_C" true))
          (for _array_element _foundwidgets
            (Widget|RemovefromParent _array_element))
          (Sequencer|Player|Play _sequenceplayer :!class /Script/MovieScene.MovieSceneSequencePlayer))))
    (:then_4
      (Collision|SetCollisionEnabled (Variables|Default|GetBox) "NoCollision"))))

(fn ConstructionScript)